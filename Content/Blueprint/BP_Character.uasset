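; Character Blueprint that switches its mesh into physics ragdoll and gets back up with a face-up or face-down montage.
; While ragdolled, Tick traces down from the pelvis and moves the capsule to an interpolated ground-based location.
; GetUp finds facing from the pelvis, aligns the actor along the pelvis-neck line and saves a pose snapshot.
; It then stops simulation, plays the montage and clears the ABP_Mannequin ragdoll flag.
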(event `self.ReceiveTick`
  (params (DeltaSeconds :type "Float (single-precision)"))
  (if (`self.IsRagdoll`)
    (`self.CalculateMeshLocation`)
    (`SceneComponent.K2_SetWorldLocation` (`self.Capsule`) (`self.MeshLocation`) false false)
    (else
      (set `self.MeshLocation` (+ (`SceneComponent.GetSocketLocation` (`self.SkeletalMesh`) "pelvis") (0.0 0.0 90.0))))))

(event `GetUp`
  (`self.CachePose`)
  (`KismetSystemLibrary.Delay` 0.2)
  (`PrimitiveComponent.SetSimulatePhysics` (`self.SkeletalMesh`) false)
  (set `self.IsRagdoll` false)
  (`|PlayMontage` (`self.SkeletalMesh`) (select `bool` (`self.Is Facing U[p`) :`false` "/PoseSnapshot/Mannequins/Animations/AM_GettingUp_FaceDown.AM_GettingUp_FaceDown" :`true` "/PoseSnapshot/Mannequins/Animations/AM_GettingUp_FaceUp.AM_GettingUp_FaceUp" :!type "AnimMontage Object Reference")
    (:`then`
      (bind _asabp_mannequin (cast `/PoseSnapshot/Mannequins/Meshes/ABP_Mannequin` (`SkeletalMeshComponent.GetAnimInstance` (`self.SkeletalMesh`))))
      (set `/PoseSnapshot/Mannequins/Meshes/ABP_Mannequin.IsRagdoll` false _asabp_mannequin))))

(event `CachePose`
  ; Cache Ragdoll Pose
  (set `self.Is Facing U[p` (`self.CalculateFacingDirection`))
  (`self.SetupGetUpOrientation`)
  (`KismetSystemLibrary.Delay` 0.0)
  (`KismetSystemLibrary.Delay` 0.0)
  (`AnimInstance.SavePoseSnapshot` (`SkeletalMeshComponent.GetAnimInstance` (`self.SkeletalMesh`)) "RagdollPose"))

(fn `CalculateFacingDirection`
  (returns (`IsFacingU[p` :type Boolean))
  (return (>= (`KismetMathLibrary.Dot_VectorVector` (`KismetMathLibrary.GetRightVector` (`SceneComponent.GetSocketRotation` (`self.SkeletalMesh`) "pelvis")) (0.0 0.0 1.0)) 0.0)))

(fn `CalculateMeshLocation`
  (bind _returnvalue (`SceneComponent.GetSocketLocation` (`self.SkeletalMesh`) "pelvis"))
  (bind (_outhit _returnvalue_2) (`KismetSystemLibrary.LineTraceSingle` _returnvalue (+ _returnvalue (* (0.0 0.0 -1.0) 100.0)) "TraceTypeQuery1"))
  (if _returnvalue_2
    (set `self.CapsuleLocation` (+ (`.Location` (`GameplayStatics.BreakHitResult` _outhit)) (0.0 0.0 90.0)))
    (else
      (set `self.CapsuleLocation` (+ (`SceneComponent.GetSocketLocation` (`self.SkeletalMesh`) "pelvis") (0.0 0.0 90.0)))))
  (set `self.MeshLocation` (`KismetMathLibrary.VInterpTo` (`self.MeshLocation`) (`self.CapsuleLocation`) (`GameplayStatics.GetWorldDeltaSeconds`) 20.0)))

(fn `SetupGetUpOrientation`
  (bind _skeletalmesh (`self.SkeletalMesh`))
  (bind _returnvalue (`SceneComponent.GetSocketLocation` _skeletalmesh "pelvis"))
  (bind _returnvalue_2 (`SceneComponent.GetSocketLocation` _skeletalmesh "neck_01"))
  (`self.K2_SetActorTransform` (`KismetMathLibrary.MakeTransform` (`self.MeshLocation`) (`KismetMathLibrary.MakeRotFromZX` (0.0 0.0 1.0) (`KismetMathLibrary.SelectVector` (- _returnvalue_2 _returnvalue) (- _returnvalue _returnvalue_2) (`self.Is Facing U[p`))))))

(fn `StartRagdoll`
  (`PrimitiveComponent.SetSimulatePhysics` (`self.SkeletalMesh`) true)
  (set `self.IsRagdoll` true)
  (bind _asabp_mannequin (cast `/PoseSnapshot/Mannequins/Meshes/ABP_Mannequin` (`SkeletalMeshComponent.GetAnimInstance` (`self.SkeletalMesh`))))
  (set `/PoseSnapshot/Mannequins/Meshes/ABP_Mannequin.IsRagdoll` true _asabp_mannequin))

(fn `UserConstructionScript`)