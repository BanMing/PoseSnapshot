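; Ch36 actor Blueprint that switches its skeletal mesh in and out of physics ragdoll.
; StartRagdoll and GetUp toggle physics simulation and IsRagdoll.
; While ragdolled, Tick traces down from the hips and moves the capsule toward a point above the ground, smoothed by interpolation.
; GetFacingDirection tests hip orientation but is not called here, and the pose snapshot, ABP_Ch36 flag and get-up montage nodes are disconnected.
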(event `self.ReceiveTick`
  (params (DeltaSeconds :type "Float (single-precision)"))
  (if (`self.IsRagdoll`)
    (`self.CalculateMeshLocation`)
    (`SceneComponent.K2_SetWorldLocation` (`self.Capsule`) (`self.MeshLocation`) false false)
    (else
      (set `self.MeshLocation` (+ (`SceneComponent.GetSocketLocation` (`self.SkeletalMesh`) "Hips") (0.0 0.0 90.0))))))

(fn `CalculateMeshLocation`
  (bind _returnvalue (`SceneComponent.GetSocketLocation` (`self.SkeletalMesh`) "Hips"))
  (bind (_outhit _returnvalue_2) (`KismetSystemLibrary.LineTraceSingle` _returnvalue (+ _returnvalue (* (0.0 0.0 -1.0) 100.0)) "TraceTypeQuery1"))
  (if _returnvalue_2
    (set `self.CapsuleLocation` (+ (`.Location` (`GameplayStatics.BreakHitResult` _outhit)) (0.0 0.0 90.0)))
    (else
      (set `self.CapsuleLocation` (+ (`SceneComponent.GetSocketLocation` (`self.SkeletalMesh`) "Hips") (0.0 0.0 90.0)))))
  (set `self.MeshLocation` (`KismetMathLibrary.VInterpTo` (`self.MeshLocation`) (`self.CapsuleLocation`) (`GameplayStatics.GetWorldDeltaSeconds`) 5.0)))

(fn `GetFacingDirection`
  (returns (IsFacing :type Boolean))
  (return (>= (`KismetMathLibrary.Dot_VectorVector` (`KismetMathLibrary.GetRightVector` (`SceneComponent.GetSocketRotation` (`self.SkeletalMesh`) "Hips")) (0.0 0.0 1.0)) 0.0)))

(fn `GetUp`
  (`PrimitiveComponent.SetSimulatePhysics` (`self.SkeletalMesh`) false)
  (set `self.IsRagdoll` false))

(fn `StartRagdoll`
  (`PrimitiveComponent.SetSimulatePhysics` (`self.SkeletalMesh`) true)
  (set `self.IsRagdoll` true))

(fn `UserConstructionScript`)